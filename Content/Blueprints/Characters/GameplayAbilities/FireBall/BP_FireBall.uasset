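; BP_FireBall is the fireball actor in the gameplay abilities folder that delivers a gameplay effect to hostile characters it touches.
; On sphere overlap, it asks its instigator character whether the other character is hostile.
; If so, the instigator applies the stored effect spec handle to that target and the fireball destroys itself.
; A timer started at BeginPlay also destroys it after a few seconds.
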(event `self.ReceiveBeginPlay`
  (`KismetSystemLibrary.K2_SetTimerDelegate` (delegate `Die`) 5.0))

(event `Die`
  (`self.K2_DestroyActor`))

(event `self.Sphere.OnComponentBeginOverlap`
  (params (OverlappedComponent :type "PrimitiveComponent Object Reference") (OtherActor :type "Actor Object Reference") (OtherComp :type "PrimitiveComponent Object Reference") (OtherBodyIndex :type Integer) (bFromSweep :type Boolean) (SweepResult :type "HitResult Structure (by ref)"))
  (bind _asbp_character_base (cast `/Game/Blueprints/Characters/BP_CharacterBase` OtherActor))
  (bind _asbp_character_base_2 (cast `/Game/Blueprints/Characters/BP_CharacterBase` (`self.GetInstigator`)))
  (bind _returnvalue (`CharacterBase.IsOtherHostile` _asbp_character_base_2 _asbp_character_base))
  (if _returnvalue
    (`CharacterBase.ApplyGameplayEffectHandle` _asbp_character_base_2 (`self.EffectSpecHandle`) (`AbilitySystemBlueprintLibrary.AbilityTargetDataFromActor` OtherActor))
    (`self.K2_DestroyActor`)))

(fn `UserConstructionScript`)
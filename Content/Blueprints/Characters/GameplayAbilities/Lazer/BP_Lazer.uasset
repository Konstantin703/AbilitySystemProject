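; BP_Lazer is a laser beam actor whose skeletal mesh changes length to match the distance to its LazerEndDetection component.
; At BeginPlay it records the original beam length from the actor location to the mesh's "end" socket.
; Each Tick it passes the difference between the current and original lengths to AnimBP_Lazer_Skeletal_Mesh as an X-axis EndBoneOffset, stretching the beam through bone animation.
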(event `self.ReceiveBeginPlay`
  (set `self.BeamOriginalLength` (`KismetMathLibrary.VSize` (- (`SceneComponent.GetSocketLocation` (`self.LazerMesh`) "end") (`self.K2_GetActorLocation`)))))

(event `self.ReceiveTick`
  (params (DeltaSeconds :type "Float (single-precision)"))
  (bind _asanim_bp_lazer_skeletal_mesh (cast `/Game/Blueprints/Characters/GameplayAbilities/Lazer/LazerAssets/AnimBP_Lazer_Skeletal_Mesh` (`SkeletalMeshComponent.GetAnimInstance` (`self.LazerMesh`))))
  (set `/Game/Blueprints/Characters/GameplayAbilities/Lazer/LazerAssets/AnimBP_Lazer_Skeletal_Mesh.EndBoneOffset` (`KismetMathLibrary.MakeVector` (- (`KismetMathLibrary.VSize` (- (`SceneComponent.K2_GetComponentLocation` (`self.LazerEndDetection`)) (`self.K2_GetActorLocation`))) (`self.BeamOriginalLength`))) _asanim_bp_lazer_skeletal_mesh))

(fn `UserConstructionScript`)
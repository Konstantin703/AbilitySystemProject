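; Player character Blueprint that keeps the primary HUD in sync with the character's health, mana and strength.
; Each attribute-changed event casts the controller to BP_PlayerControllerBase and sets the matching glass-ball widget in its PrimaryUI to the current value divided by its maximum.
; The construction script only calls the parent implementation.
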(event `self.BP_OnHealthChanged`
  (params (Health :type "Float (single-precision)") (MaxHealth :type "Float (single-precision)"))
  (bind _asbp_player_controller_base (cast `/Game/Blueprints/BP_PlayerControllerBase` (`self.GetController`)))
  (`/Game/UI/WidgetsUI/UI_GlassBall.SetPercentage` (`/Game/UI/WidgetsUI/UI_Primary.UI_HealthGlassBall` (`/Game/Blueprints/BP_PlayerControllerBase.PrimaryUI` _asbp_player_controller_base)) (/ Health MaxHealth)))

(event `self.BP_OnManaChanged`
  (params (Mana :type "Float (single-precision)") (MaxMana :type "Float (single-precision)"))
  (bind _asbp_player_controller_base (cast `/Game/Blueprints/BP_PlayerControllerBase` (`self.GetController`)))
  (`/Game/UI/WidgetsUI/UI_GlassBall.SetPercentage` (`/Game/UI/WidgetsUI/UI_Primary.UI_ManaGlassBall` (`/Game/Blueprints/BP_PlayerControllerBase.PrimaryUI` _asbp_player_controller_base)) (/ Mana MaxMana)))

(event `self.BP_OnStrengthChanged`
  (params (Strength :type "Float (single-precision)") (MaxStrength :type "Float (single-precision)"))
  (bind _asbp_player_controller_base (cast `/Game/Blueprints/BP_PlayerControllerBase` (`self.GetController`)))
  (`/Game/UI/WidgetsUI/UI_GlassBall.SetPercentage` (`/Game/UI/WidgetsUI/UI_Primary.UI_StrengthGlassBall` (`/Game/Blueprints/BP_PlayerControllerBase.PrimaryUI` _asbp_player_controller_base)) (/ Strength MaxStrength)))

(fn `UserConstructionScript`
  (`parent.UserConstructionScript`))